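; BP_PuzzleRotator is an interactable puzzle piece whose picture mesh turns a quarter turn each time it is used.
; The construction script applies the configurable PictureMesh to the Picture component.
; E-Interact plays a timeline, ignored while already playing, that lerps the relative pitch down by 90 degrees.
; On finish it stores the new pitch in PictureRotation as the base for the next turn.
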(event `/Game/Room3/KPBlueprints/BPI_Interact.E-Interact`
  (bind (_picturerotation_roll _picturerotation_pitch) (`KismetMathLibrary.BreakRotator` (`self.PictureRotation`)))
  (if (not (`TimelineComponent.IsPlaying` (`self.TL_Timeline`)))
    (bind (_direction _alpha) (`Timeline|TL_Timeline` :!via `PlayFromStart`)
      (:`Update`
        (bind _returnvalue (`KismetMathLibrary.Lerp` _picturerotation_pitch (- _picturerotation_pitch 90.0) _alpha))
        (`SceneComponent.K2_SetRelativeRotation` (`self.Picture`) (`KismetMathLibrary.MakeRotator` 0.0 _returnvalue) false false))
      (:`Finished`
        (set `self.PictureRotation` (`KismetMathLibrary.MakeRotator` 0.0 _returnvalue))))))

(fn `UserConstructionScript`
  (`StaticMeshComponent.SetStaticMesh` (`self.Picture`) (`self.PictureMesh`)))
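; Room 3 keypad actor that the player interacts with to enter a code.
; Two spheres, sized in the construction script, swap outer and inner interact icons by player proximity.
; Tick polls the player's IsInteracting and HitActor, then blends the view to the keypad, locks look and movement, enables the cursor and adds WBP_Keypad.
; Only Button1 is wired, appending "1", updating the widget text and printing whether input matches CorrectCode.
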(event `self.innerSphereCollision.OnComponentBeginOverlap`
  (params (OverlappedComponent :type "PrimitiveComponent Object Reference") (OtherActor :type "Actor Object Reference") (OtherComp :type "PrimitiveComponent Object Reference") (OtherBodyIndex :type Integer) (bFromSweep :type Boolean) (SweepResult :type "HitResult Structure (by ref)"))
  ;[0 0.1714 0.5395 0.502] Display Icon
  (if (== OtherActor (`GameplayStatics.GetPlayerCharacter` 0))
    (`SceneComponent.SetVisibility` (`self.innerInteractIcon`) true false)
    (`SceneComponent.SetVisibility` (`self.outerInteractIcon`) false false)))

(event `self.ReceiveBeginPlay`
  ;[0 0.1714 0.5395 0.502] Interact
  (bind _asbp_first_person_character (cast `/Game/FirstPerson/Blueprints/BP_FirstPersonCharacter` (`GameplayStatics.GetPlayerCharacter` 0)))
  (set `self.BP Player Ref` _asbp_first_person_character)
  (bind _returnvalue (`|CreateWidget` "/Game/Room3/KPBlueprints/WBP_Keypad.WBP_Keypad_C"))
  (set `self.Keypad REF` _returnvalue))

(event `self.ReceiveTick`
  (params (DeltaSeconds :type "Float (single-precision)"))
  (bind _returnvalue (`GameplayStatics.GetPlayerController` 0))
  (bind _bp_player_ref (`self.BP Player Ref`))
  ;[0 0.1714 0.5395 0.502] Interact
  (if (and (`/Game/FirstPerson/Blueprints/BP_FirstPersonCharacter.Is Interacting?` _bp_player_ref) (== (`/Game/FirstPerson/Blueprints/BP_FirstPersonCharacter.Hit Actor` _bp_player_ref) self))
    (`PlayerController.SetViewTargetWithBlend` _returnvalue self 0.3 "VTBlend_Linear" 0.0 false)
    (`Controller.SetIgnoreLookInput` _returnvalue true)
    (set `PlayerController.bEnableClickEvents` true _returnvalue)
    (set `PlayerController.bShowMouseCursor` true _returnvalue)
    (`CharacterMovementComponent.DisableMovement` (`Character.CharacterMovement` (`GameplayStatics.GetPlayerCharacter` 0)))
    (`UserWidget.AddToViewport` (`self.Keypad REF`) 0)))

(event `self.innerSphereCollision.OnComponentEndOverlap`
  (params (OverlappedComponent :type "PrimitiveComponent Object Reference") (OtherActor :type "Actor Object Reference") (OtherComp :type "PrimitiveComponent Object Reference") (OtherBodyIndex :type Integer))
  ;[0 0.1714 0.5395 0.502] Display Icon
  (if (== (`GameplayStatics.GetPlayerCharacter` 0) OtherActor)
    (`SceneComponent.SetVisibility` (`self.innerInteractIcon`) false false)
    (`SceneComponent.SetVisibility` (`self.outerInteractIcon`) true false)))

(event `Interacted Alert`
  ;[0.000998 0.5448 0.01441 0.5] Testing Statements
  (`KismetSystemLibrary.PrintString` "Interacted with Item"))

(event `self.outerSphereCollision.OnComponentBeginOverlap`
  (params (OverlappedComponent :type "PrimitiveComponent Object Reference") (OtherActor :type "Actor Object Reference") (OtherComp :type "PrimitiveComponent Object Reference") (OtherBodyIndex :type Integer) (bFromSweep :type Boolean) (SweepResult :type "HitResult Structure (by ref)"))
  ;[0 0.1714 0.5395 0.502] Display Icon
  (if (== OtherActor (`GameplayStatics.GetPlayerCharacter` 0))
    (`SceneComponent.SetVisibility` (`self.outerInteractIcon`) true false)))

(event `self.button1.OnClicked`
  (params (TouchedComponent :type "PrimitiveComponent Object Reference") (ButtonPressed :type "Key Structure"))
  (bind _output_get (set `self.Input ` (`KismetStringLibrary.Concat_StrStr` (`self.Input `) "1")))
  (set `self.Length of Code` (+ (`self.Length of Code`) 1))
  (`TextBlock.SetText` (`/Game/Room3/KPBlueprints/WBP_Keypad.Codetext` (`self.Keypad REF`)) (`KismetTextLibrary.Conv_StringToText` _output_get))
  (if (`KismetStringLibrary.EqualEqual_StrStr` (`self.Input `) (`self.Correct Code`))
    (`KismetSystemLibrary.PrintString` "CORRECT" true true (struct :`R` 1.0 :`G` 0.002207 :`B` 0.004059 :`A` 1.0))
    (else
      (`KismetSystemLibrary.PrintString` "INCORRECT" true true (struct :`R` 0.125343 :`G` 1.0 :`A` 1.0)))))

(event `self.outerSphereCollision.OnComponentEndOverlap`
  (params (OverlappedComponent :type "PrimitiveComponent Object Reference") (OtherActor :type "Actor Object Reference") (OtherComp :type "PrimitiveComponent Object Reference") (OtherBodyIndex :type Integer))
  ;[0 0.1714 0.5395 0.502] Display Icon
  (if (== (`GameplayStatics.GetPlayerCharacter` 0) OtherActor)
    (`SceneComponent.SetVisibility` (`self.outerInteractIcon`) false false)))

(fn `UserConstructionScript`
  (`SphereComponent.SetSphereRadius` (`self.innerSphereCollision`) (`self.innerSphereRadius`) true)
  (`SphereComponent.SetSphereRadius` (`self.outerSphereCollision`) (`self.outterSphereRadius`) true))
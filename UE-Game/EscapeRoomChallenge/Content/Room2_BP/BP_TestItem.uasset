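; BP_TestItem is a test interactable item that shows proximity icons to the player and prints a debug message when interacted with.
; Two sphere collisions, sized in the construction script from radius variables, swap an outer icon for an inner icon as the player approaches.
; Every Tick it polls the cached BP_FirstPersonCharacter and fires InteractedAlert while that character is interacting with this actor as its HitActor.
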(event `self.innerSphereCollision.OnComponentBeginOverlap`
  (params (OverlappedComponent :type "PrimitiveComponent Object Reference") (OtherActor :type "Actor Object Reference") (OtherComp :type "PrimitiveComponent Object Reference") (OtherBodyIndex :type Integer) (bFromSweep :type Boolean) (SweepResult :type "HitResult Structure (by ref)"))
  ;[0 0.1714 0.5395 0.502] Display Icon
  (if (== OtherActor (`GameplayStatics.GetPlayerCharacter` 0))
    (`SceneComponent.SetVisibility` (`self.innerInteractIcon`) true false)
    (`SceneComponent.SetVisibility` (`self.outerInteractIcon`) false false)))

(event `self.ReceiveBeginPlay`
  ;[0 0.1714 0.5395 0.502] Interact
  (bind _asbp_first_person_character (cast `/Game/FirstPerson/Blueprints/BP_FirstPersonCharacter` (`GameplayStatics.GetPlayerCharacter` 0)))
  (set `self.BP Player Ref` _asbp_first_person_character))

(event `self.ReceiveTick`
  (params (DeltaSeconds :type "Float (single-precision)"))
  (bind _bp_player_ref (`self.BP Player Ref`))
  ;[0 0.1714 0.5395 0.502] Interact
  (if (and (`/Game/FirstPerson/Blueprints/BP_FirstPersonCharacter.Is Interacting?` _bp_player_ref) (== (`/Game/FirstPerson/Blueprints/BP_FirstPersonCharacter.Hit Actor` _bp_player_ref) self))
    (`self.Interacted Alert`)))

(event `self.innerSphereCollision.OnComponentEndOverlap`
  (params (OverlappedComponent :type "PrimitiveComponent Object Reference") (OtherActor :type "Actor Object Reference") (OtherComp :type "PrimitiveComponent Object Reference") (OtherBodyIndex :type Integer))
  ;[0 0.1714 0.5395 0.502] Display Icon
  (if (== (`GameplayStatics.GetPlayerCharacter` 0) OtherActor)
    (`SceneComponent.SetVisibility` (`self.innerInteractIcon`) false false)
    (`SceneComponent.SetVisibility` (`self.outerInteractIcon`) true false)))

(event `Interacted Alert`
  ;[0.000998 0.5448 0.01441 0.5] Testing Statements
  (`KismetSystemLibrary.PrintString` "Interacted with Item"))

(event `self.outerSphereCollision.OnComponentBeginOverlap`
  (params (OverlappedComponent :type "PrimitiveComponent Object Reference") (OtherActor :type "Actor Object Reference") (OtherComp :type "PrimitiveComponent Object Reference") (OtherBodyIndex :type Integer) (bFromSweep :type Boolean) (SweepResult :type "HitResult Structure (by ref)"))
  ;[0 0.1714 0.5395 0.502] Display Icon
  (if (== OtherActor (`GameplayStatics.GetPlayerCharacter` 0))
    (`SceneComponent.SetVisibility` (`self.outerInteractIcon`) true false)))

(event `self.outerSphereCollision.OnComponentEndOverlap`
  (params (OverlappedComponent :type "PrimitiveComponent Object Reference") (OtherActor :type "Actor Object Reference") (OtherComp :type "PrimitiveComponent Object Reference") (OtherBodyIndex :type Integer))
  ;[0 0.1714 0.5395 0.502] Display Icon
  (if (== (`GameplayStatics.GetPlayerCharacter` 0) OtherActor)
    (`SceneComponent.SetVisibility` (`self.outerInteractIcon`) false false)))

(fn `UserConstructionScript`
  (`SphereComponent.SetSphereRadius` (`self.innerSphereCollision`) (`self.innerSphereRadius`) true)
  (`SphereComponent.SetSphereRadius` (`self.outerSphereCollision`) (`self.outterSphereRadius`) true))
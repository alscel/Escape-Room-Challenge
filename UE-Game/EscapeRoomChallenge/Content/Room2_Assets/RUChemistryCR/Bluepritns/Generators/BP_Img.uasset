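; BP_Img is an actor that displays a configurable image on a plane mesh.
; Its construction script either applies the MalbertMI material when IsMalbert is set, or creates a dynamic instance of M_Imgs fed with the ImgTexture and NormalTexture as albedo and normal maps.
; The event graph holds only disabled placeholder events, so it has no runtime logic.
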(fn `UserConstructionScript`
  (if (`self.IsMalbert`)
    (`PrimitiveComponent.SetMaterial` (`self.Plane`) 0 (`self.Malbert MI`))
    (else
      (bind _returnvalue (`PrimitiveComponent.CreateDynamicMaterialInstance` (`self.Plane`) 0 "/Game/Room2_Assets/RUChemistryCR/Materials/Other/M_Imgs.M_Imgs" "None"))
      (`MaterialInstanceDynamic.SetTextureParameterValue` _returnvalue "Albedo Texture" (`self.Img Texture`))
      (`MaterialInstanceDynamic.SetTextureParameterValue` _returnvalue "Normal Texture" (`self.Normal Texture`)))))